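; Trigger actor that toggles the colour of a set of spotlights each time an actor begins overlapping it.
; A FlipFlop on the overlap event alternates between two colours, looping over the Spotlights array to apply the current one to each SpotLight component.
; Any overlapping actor triggers the switch, and ending the overlap does not revert it.
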(event `self.ReceiveActorBeginOverlap`
  (params (OtherActor :type "Actor Object Reference"))
  (`/Engine/EditorBlueprintResources/StandardMacros.FlipFlop`
    (:`A`
      (for _array_element (`self.Spotlights`)
        (`LightComponent.SetLightColor` (`/Game/MyStuff/SpotlghtSystem/BP_Spotlight.SpotLight` _array_element) (`self.New Light Color`) true)))
    (:`B`
      (for _array_element_2 (`self.Spotlights`)
        (`LightComponent.SetLightColor` (`/Game/MyStuff/SpotlghtSystem/BP_Spotlight.SpotLight` _array_element_2) (`self.NewLightColourB`) true)))))

(fn `UserConstructionScript`)